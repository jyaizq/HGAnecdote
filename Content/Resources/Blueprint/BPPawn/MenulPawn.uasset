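; MenulPawn is the menu pawn that shows a rotatable product preview and opens the MenulUI widget with a visible mouse cursor.
; UpdataProMesh looks up a ProDataTable row by ID, lazily spawns MenulPro_Bp at the MenulProLoc actor found on BeginPlay, then applies the row's mesh and relative transform.
; Input axes rotate the preview, yawing the whole actor and pitching its MeshPich component.
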(event EventBeginPlay
  (bind _returnvalue (Game|GetPlayerController 0))
  (CallFunction|Init)
  (Input|SetInputModeGameandUI _returnvalue 0 "LockInFullscreen" true)
  (bind _returnvalue_2 (UserInterface|CreateWidget "/Game/Resources/Blueprint/UserBlueprint/MenulUI.MenulUI_C" _returnvalue))
  (UserInterface|Viewport|AddtoViewport _returnvalue_2 0)
  (Variables|/Script/Engine.PlayerController|SetbShowMouseCursor _returnvalue true))

(event Collision|EventActorBeginOverlap
  (params (OtherActor :type Actor%20Object%20Reference)))

(event EventTick
  (params (DeltaSeconds :type Float%20%28single-precision%29)))

(event Input|AxisEvents|InputAxisInputXAxis
  (params (AxisValue :type Float%20%28single-precision%29))
  (if (!= (stale Input|AxisEvents|InputAxisRightMouseClick AxisValue) 0.0)
    (Class|Actor|AddActorWorldRotation (Variables|Default|GetMenulPro) (Math|Rotator|MakeRotator 0.0 0.0 (* AxisValue (Variables|Default|Getspeed))))))

(event Input|AxisEvents|InputAxisInputYAxis
  (params (AxisValue :type Float%20%28single-precision%29))
  (if (!= (stale Input|AxisEvents|InputAxisRightMouseClick AxisValue) 0.0)
    (Transformation|AddLocalRotation (Variables|/Game/Resources/Blueprint/BPActor/MenulPro_Bp.MenulPro_Bp_C|GetMeshPich (Variables|Default|GetMenulPro)) (Math|Rotator|MakeRotator 0.0 (* AxisValue (Variables|Default|Getspeed)) 0.0) false false)))

(event Input|AxisEvents|InputAxisRightMouseClick
  (params (AxisValue :type Float%20%28single-precision%29)))

(fn ConstructionScript)

(fn Init
  (bind _outactors (Actor|GetAllActorsOfClass "/Game/Resources/Blueprint/BPActor/MenulProLoc.MenulProLoc_C"))
  (if (>= (Utilities|Array|Length _outactors) 1)
    (Variables|Default|SetMenulProLocation (Utilities|Array|Get(acopy) _outactors))))

(fn LoadMenulPro
  (bind _returnvalue (Game|SpawnActorfromClass "/Game/Resources/Blueprint/BPActor/MenulPro_Bp.MenulPro_Bp_C" (Transformation|GetActorTransform (Variables|Default|GetMenulProLocation)) "Undefined" 0 0))
  (Variables|Default|SetMenulPro _returnvalue))

(fn UpdataProMesh
  (params (ProID :type Name))
  (bind _menulpro (Variables|Default|GetMenulPro))
  (bind _staticmesh (Variables|/Game/Resources/Blueprint/BPActor/MenulPro_Bp.MenulPro_Bp_C|GetStaticMesh _menulpro))
  (bind _returnvalue (Utilities|GetDataTableRow "/Game/Resources/Blueprint/DataTable/ProDataTable.ProDataTable" ProID)
    (:then
      (Utilities|IsValid _menulpro
        (:Is%20Valid
          _)
        (:Is%20Not%20Valid
          (CallFunction|LoadMenulPro)))
      (Components|StaticMesh|SetStaticMesh _staticmesh (.ProMesh (Utilities|Struct|BreakProInfo _returnvalue)))
      (Transformation|SetRelativeTransform _staticmesh (Math|Transform|MakeTransform (.RelativeLoc (Utilities|Struct|BreakProInfo _returnvalue)) (.RelativeRot (Utilities|Struct|BreakProInfo _returnvalue)) (.RelativeScale (Utilities|Struct|BreakProInfo _returnvalue))) false false)
      (Default|RestSelf _menulpro))))